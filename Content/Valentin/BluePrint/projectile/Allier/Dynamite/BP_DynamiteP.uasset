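; BP_DynamiteP is an allied dynamite projectile that turns into a dynamite zone on impact.
; Tick nudges its pitch by a tiny fixed step each frame, independent of delta time.
; On overlap with a path slot, path-edge slot or test enemy, it spawns BP_ZoneDynamite at its location and destroys itself.
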(event `self.ReceiveTick`
  (params (DeltaSeconds :type "Float (single-precision)"))
  (bind (_returnvalue_roll _returnvalue_pitch) (`KismetMathLibrary.BreakRotator` (`self.K2_GetActorRotation`)))
  (`self.K2_SetActorRotation` (`KismetMathLibrary.MakeRotator` 0.0 (+ _returnvalue_pitch 0.001))))

(event `self.ReceiveActorBeginOverlap`
  (params (OtherActor :type "Actor Object Reference"))
  (bind _returnvalue (`self.K2_GetActorLocation`))
  (`|ExecutionSequence`
    (:`then_0`
      (cast `/Game/Valentin/BluePrint/BP_SlotChemin` OtherActor)
      (`|SpawnActorFromClass` "/Game/Valentin/BluePrint/projectile/Allier/Dynamite/BP_ZoneDynamite.BP_ZoneDynamite_C" (`KismetMathLibrary.Conv_VectorToTransform` _returnvalue) "Undefined" "OverrideRootScale" null null)
      (`self.K2_DestroyActor`))
    (:`then_1`
      (cast `/Game/Valentin/BluePrint/BP_SlotBordChemin` OtherActor)
      (`|SpawnActorFromClass` "/Game/Valentin/BluePrint/projectile/Allier/Dynamite/BP_ZoneDynamite.BP_ZoneDynamite_C" (`KismetMathLibrary.Conv_VectorToTransform` _returnvalue) "Undefined" "OverrideRootScale" null null)
      (`self.K2_DestroyActor`))
    (:`then_2`
      (cast `/Game/Valentin/BluePrint/BP_TestEnemie` OtherActor)
      (`|SpawnActorFromClass` "/Game/Valentin/BluePrint/projectile/Allier/Dynamite/BP_ZoneDynamite.BP_ZoneDynamite_C" (`KismetMathLibrary.Conv_VectorToTransform` _returnvalue) "Undefined" "OverrideRootScale" null null)
      (`self.K2_DestroyActor`))))

(fn `UserConstructionScript`)