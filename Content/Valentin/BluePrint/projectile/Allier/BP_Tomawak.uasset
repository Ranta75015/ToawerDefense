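; BP_Tomawak is a damage projectile, in the ally projectile folder, that hits BP_TestEnemie actors.
; Every tick it copies MultiplicateurInd from the player's BP_FinalPlayer pawn into its own multiplier.
; On overlap with an enemy it applies ProjectileDamage scaled by that multiplier, then destroys itself.
; A timer set at BeginPlay destroys it after a few seconds if it hits nothing.
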(event `self.ReceiveTick`
  (params (DeltaSeconds :type "Float (single-precision)"))
  (bind _asbp_final_player (cast `/Game/Valentin/BluePrint/BP_FinalPlayer` (`GameplayStatics.GetPlayerPawn` 0)))
  (set `self.Multiplicatore` (`/Game/Valentin/BluePrint/BP_FinalPlayer.Multiplicateur Ind` _asbp_final_player)))

(event `self.ReceiveActorBeginOverlap`
  (params (OtherActor :type "Actor Object Reference"))
  (bind _asbp_test_enemie (cast `/Game/Valentin/BluePrint/Ennemie/BP_TestEnemie` OtherActor))
  (`GameplayStatics.ApplyDamage` _asbp_test_enemie (* (`self.Projectile Damage`) (`self.Multiplicatore`)))
  (`self.K2_DestroyActor`))

(event `self.ReceiveBeginPlay`
  (`KismetSystemLibrary.K2_SetTimerDelegate` (delegate `destroy`) 5.0 true))

(event `destroy`
  (`self.K2_DestroyActor`))

(fn `UserConstructionScript`)