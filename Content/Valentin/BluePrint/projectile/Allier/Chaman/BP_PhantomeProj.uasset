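; Phantom projectile of the allied shaman that turns into a BP_ZoneShaman area when it overlaps a path slot, path-edge slot or enemy.
; On spawn it randomly shows a crow, rabbit or wolf, with the wolf twice as likely, and starts a five-second self-destruct timer.
; Each tick it copies the player's multiplier, which it passes to the spawned zone; the impact Niagara component is added after DestroyActor.
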(event `self.ReceiveTick`
  (params (DeltaSeconds :type "Float (single-precision)"))
  (bind _asbp_final_player (cast `/Game/Valentin/BluePrint/BP_FinalPlayer` (`GameplayStatics.GetPlayerPawn` 0)))
  (set `self.Multiplicatore` (`/Game/Valentin/BluePrint/BP_FinalPlayer.Multiplicateur Ind` _asbp_final_player)))

(event `self.ReceiveActorBeginOverlap`
  (params (OtherActor :type "Actor Object Reference"))
  (bind _returnvalue (`self.K2_GetActorLocation`))
  (`|ExecutionSequence`
    (:`then_0`
      (cast `/Game/Valentin/BluePrint/BP_SlotChemin` OtherActor)
      (bind _returnvalue_2 (`|SpawnActorFromClass` "/Game/Valentin/BluePrint/projectile/Allier/Chaman/BP_ZoneShaman.BP_ZoneShaman_C" (`KismetMathLibrary.Conv_VectorToTransform` _returnvalue) "Undefined" "OverrideRootScale" null null))
      (`self.K2_DestroyActor`)
      (`AddComponent|NODE_AddNiagaraComponent-0` :`bManualAttachment` true :`RelativeTransform` (`self.GetTransform`))
      (set `/Game/Valentin/BluePrint/projectile/Allier/Chaman/BP_ZoneShaman.Multiplicatore` (`self.Multiplicatore`) _returnvalue_2))
    (:`then_1`
      (cast `/Game/Valentin/BluePrint/BP_SlotBordChemin` OtherActor)
      (bind _returnvalue_3 (`|SpawnActorFromClass` "/Game/Valentin/BluePrint/projectile/Allier/Chaman/BP_ZoneShaman.BP_ZoneShaman_C" (`KismetMathLibrary.Conv_VectorToTransform` _returnvalue) "Undefined" "OverrideRootScale" null null))
      (`self.K2_DestroyActor`)
      (`AddComponent|NODE_AddNiagaraComponent-1` :`bManualAttachment` true :`RelativeTransform` (`self.GetTransform`))
      (set `/Game/Valentin/BluePrint/projectile/Allier/Chaman/BP_ZoneShaman.Multiplicatore` (`self.Multiplicatore`) _returnvalue_3))
    (:`then_2`
      (cast `/Game/Valentin/BluePrint/Ennemie/BP_TestEnemie` OtherActor)
      (bind _returnvalue_4 (`|SpawnActorFromClass` "/Game/Valentin/BluePrint/projectile/Allier/Chaman/BP_ZoneShaman.BP_ZoneShaman_C" (`KismetMathLibrary.Conv_VectorToTransform` _returnvalue) "Undefined" "OverrideRootScale" null null))
      (`self.K2_DestroyActor`)
      (`AddComponent|NODE_AddNiagaraComponent-2` :`bManualAttachment` true :`RelativeTransform` (`self.GetTransform`))
      (set `/Game/Valentin/BluePrint/projectile/Allier/Chaman/BP_ZoneShaman.Multiplicatore` (`self.Multiplicatore`) _returnvalue_4))))

(event `self.ReceiveBeginPlay`
  (`self.Random Fantome`)
  (`KismetSystemLibrary.K2_SetTimerDelegate` (delegate `destroy`) 5.0 true))

(event `destroy`
  (`self.K2_DestroyActor`))

(fn `Random Fantome`
  (set `self.Random` (`KismetMathLibrary.RandomIntegerInRange` 1 4))
  (if (== (`self.Random`) 1)
    (`SceneComponent.SetHiddenInGame` (`self.LE_CORBEAU`) false false)
    (`SceneComponent.SetHiddenInGame` (`self.LE_LAPIN`) true false)
    (`SceneComponent.SetHiddenInGame` (`self.LE_LOUP`) true false)
    (elif (== (`self.Random`) 2)
      (`SceneComponent.SetHiddenInGame` (`self.LE_CORBEAU`) true false)
      (`SceneComponent.SetHiddenInGame` (`self.LE_LAPIN`) false false)
      (`SceneComponent.SetHiddenInGame` (`self.LE_LOUP`) true false)
      (else
        (`SceneComponent.SetHiddenInGame` (`self.LE_CORBEAU`) true false)
        (`SceneComponent.SetHiddenInGame` (`self.LE_LAPIN`) true false)
        (`SceneComponent.SetHiddenInGame` (`self.LE_LOUP`) false false)))))

(fn `UserConstructionScript`)