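; BP_bouler is an allied projectile that turns into a BP_ZoneBouler zone on impact.
; Every tick it copies MultiplicateurFr from BP_FinalPlayer into its Multiplicatore.
; Overlapping a path slot, path-edge slot or BP_TestEnemie spawns the zone at its location and destroys the projectile.
; The spawned zone receives the stored multiplier.
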(event `self.ReceiveTick`
  (params (DeltaSeconds :type "Float (single-precision)"))
  (bind _asbp_final_player (cast `/Game/Valentin/BluePrint/BP_FinalPlayer` (`GameplayStatics.GetPlayerPawn` 0)))
  (set `self.Multiplicatore` (`/Game/Valentin/BluePrint/BP_FinalPlayer.Multiplicateur Fr` _asbp_final_player)))

(event `self.ReceiveActorBeginOverlap`
  (params (OtherActor :type "Actor Object Reference"))
  (bind _returnvalue (`self.K2_GetActorLocation`))
  (`|ExecutionSequence`
    (:`then_0`
      (cast `/Game/Valentin/BluePrint/BP_SlotChemin` OtherActor)
      (bind _returnvalue_2 (`|SpawnActorFromClass` "/Game/Valentin/BluePrint/projectile/Allier/Bouler/BP_ZoneBouler.BP_ZoneBouler_C" (`KismetMathLibrary.Conv_VectorToTransform` _returnvalue) "Undefined" "OverrideRootScale" null null))
      (`self.K2_DestroyActor`)
      (set `/Game/Valentin/BluePrint/projectile/Allier/Bouler/BP_ZoneBouler.Multiplicatore` (`self.Multiplicatore`) _returnvalue_2))
    (:`then_1`
      (cast `/Game/Valentin/BluePrint/BP_SlotBordChemin` OtherActor)
      (bind _returnvalue_3 (`|SpawnActorFromClass` "/Game/Valentin/BluePrint/projectile/Allier/Bouler/BP_ZoneBouler.BP_ZoneBouler_C" (`KismetMathLibrary.Conv_VectorToTransform` _returnvalue) "Undefined" "OverrideRootScale" null null))
      (`self.K2_DestroyActor`)
      (set `/Game/Valentin/BluePrint/projectile/Allier/Bouler/BP_ZoneBouler.Multiplicatore` (`self.Multiplicatore`) _returnvalue_3))
    (:`then_2`
      (cast `/Game/Valentin/BluePrint/BP_TestEnemie` OtherActor)
      (bind _returnvalue_4 (`|SpawnActorFromClass` "/Game/Valentin/BluePrint/projectile/Allier/Bouler/BP_ZoneBouler.BP_ZoneBouler_C" (`KismetMathLibrary.Conv_VectorToTransform` _returnvalue) "Undefined" "OverrideRootScale" null null))
      (`self.K2_DestroyActor`)
      (set `/Game/Valentin/BluePrint/projectile/Allier/Bouler/BP_ZoneBouler.Multiplicatore` (`self.Multiplicatore`) _returnvalue_4))))

(fn `UserConstructionScript`)