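; BP_AmoEnnemie is an enemy projectile that damages the player's defensive structures on contact.
; On overlap, a Sequence tests the other actor against BP_TestTour, BP_ShootWall and BP_TestDéfense through separate casts; a match receives the same fixed damage and the projectile destroys itself.
; A timer started on BeginPlay also destroys it after a few seconds.
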(event `self.ReceiveBeginPlay`
  (`KismetSystemLibrary.K2_SetTimerDelegate` (delegate `destroy`) 5.0 true))

(event `self.ReceiveActorBeginOverlap`
  (params (OtherActor :type "Actor Object Reference"))
  (`|ExecutionSequence`
    (:`then_0`
      (bind _asbp_test_tour (cast `/Game/Valentin/BluePrint/Tour/BP_TestTour` OtherActor))
      (`GameplayStatics.ApplyDamage` _asbp_test_tour 2.0)
      (`self.K2_DestroyActor`))
    (:`then_1`
      (bind _asbp_shoot_wall (cast `/Game/Valentin/BluePrint/Trap/BP_ShootWall` OtherActor))
      (`GameplayStatics.ApplyDamage` _asbp_shoot_wall 2.0)
      (`self.K2_DestroyActor`))
    (:`then_2`
      (bind `_asbp_test_défense` (cast `/Game/Valentin/BluePrint/BP_TestDéfense` OtherActor))
      (`GameplayStatics.ApplyDamage` `_asbp_test_défense` 2.0)
      (`self.K2_DestroyActor`))))

(event `destroy`
  (`self.K2_DestroyActor`))

(fn `UserConstructionScript`)