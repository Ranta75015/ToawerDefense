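; BP_SlotBordChemin is a clickable tower slot, named as a path-edge slot, where the player builds or upgrades a tower.
; Hovering the cube shifts the actor along its up vector as feedback, and leaving shifts it back.
; Releasing a click on it opens the build or upgrade widget depending on IsBuild, passing itself as the slot.
; Every Tick checks MyTower and clears IsBuild once the tower is no longer valid.
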(event `self.Cube.OnBeginCursorOver`
  (params (TouchedComponent :type "PrimitiveComponent Object Reference"))
  ;[1 0.9385 0] Feed Back si la souris survole
  (if (not (`self.Is over?`))
    (set `self.Is over?` true)
    (`self.K2_SetActorLocation` (+ (`self.K2_GetActorLocation`) (* (`self.GetActorUpVector`) (`self.Up`))) false true)))

(event `Chek vie tour`
  (`/Engine/EditorBlueprintResources/StandardMacros.IsValid` (`self.My Tower`)
    (:`Is Not Valid`
      (set `self.Is Build?` false))))

(event `self.Cube.OnEndCursorOver`
  (params (TouchedComponent :type "PrimitiveComponent Object Reference"))
  ;[1 0.9385 0] Feed Back si la souris survole
  (if (`self.Is over?`)
    (set `self.Is over?` false)
    (`self.K2_SetActorLocation` (- (`self.K2_GetActorLocation`) (* (`self.GetActorUpVector`) (`self.Down`))) false true)))

(event `self.Cube.OnReleased`
  (params (TouchedComponent :type "PrimitiveComponent Object Reference") (ButtonReleased :type "Key Structure"))
  (if (`self.Is Build?`)
    (bind _returnvalue (`|CreateWidget` "/Game/Valentin/Ui/UI_Tower/UI_AmelirationTour.UI_AmelirationTour_C"))
    (`UserWidget.AddToViewport` _returnvalue 0)
    (set `/Game/Valentin/Ui/UI_Tower/UI_AmelirationTour.Slott` self _returnvalue)
    (else
      (bind _returnvalue_2 (`|CreateWidget` "/Game/Valentin/Ui/UI_Tower/UI_BuildTower.UI_BuildTower_C"))
      (`UserWidget.AddToViewport` _returnvalue_2 0)
      (set `/Game/Valentin/Ui/UI_Tower/UI_BuildTower.Slott` self _returnvalue_2))))

(event `self.ReceiveTick`
  (params (DeltaSeconds :type "Float (single-precision)"))
  (`self.Chek vie tour`))

(fn `UserConstructionScript`)