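; BP_SlotChemin is a path slot actor that the player clicks to open a road build menu.
; Cursor hover over its Cube raises the actor along its up vector, and leaving lowers it, with IsOver guarding against repeated moves.
; Releasing a click on an unbuilt slot creates a UI_BuildOnRoad widget, adds it to the viewport and passes itself as the target slot.
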(event `self.Cube.OnBeginCursorOver`
  (params (TouchedComponent :type "PrimitiveComponent Object Reference"))
  ;[1 0.9385 0] Feed Back si la souris survole
  (if (not (`self.Is over?`))
    (`self.K2_SetActorLocation` (+ (`self.K2_GetActorLocation`) (* (`self.GetActorUpVector`) (`self.Up`))))
    (set `self.Is over?` true)))

(event `self.Cube.OnEndCursorOver`
  (params (TouchedComponent :type "PrimitiveComponent Object Reference"))
  ;[1 0.9385 0] Feed Back si la souris survole
  (if (`self.Is over?`)
    (`self.K2_SetActorLocation` (- (`self.K2_GetActorLocation`) (* (`self.GetActorUpVector`) (`self.Down`))))
    (set `self.Is over?` false)))

(event `self.Cube.OnReleased`
  (params (TouchedComponent :type "PrimitiveComponent Object Reference") (ButtonReleased :type "Key Structure"))
  (if (not (`self.Is Build?`))
    (bind _returnvalue (`|CreateWidget` "/Game/Valentin/Ui/UI_Tower/UI_BuildOnRoad.UI_BuildOnRoad_C"))
    (`UserWidget.AddToViewport` _returnvalue 0)
    (set `/Game/Valentin/Ui/UI_Tower/UI_BuildOnRoad.Slott` self _returnvalue)))

(fn `UserConstructionScript`)