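; Spawn manager that sends waves of AI enemies on a looping timer once the tutorial is finished.
; Each tick spawns two enemies at random SpawnPoint entries, rising to three and four as the tick counter grows, favoring BP_Fantassin over BP_FusilsBritish.
; TimeSpawn decreases each tick, but the timer is never reset, so its interval stays fixed.
; Spawn logic is duplicated inline, leaving the stub RandomEnemy unused.
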(event `self.ReceiveBeginPlay`
  (`KismetSystemLibrary.K2_SetTimerDelegate` (delegate `Sapwn`) (`self.Time spawn`) true))

(event `Sapwn`
  (bind (_returnvalue_location _returnvalue_rotation) (`KismetMathLibrary.BreakTransform` (`self.GetTransform` (`self.Random Spawn`))))
  (bind (_returnvalue_location_2 _returnvalue_rotation_2) (`KismetMathLibrary.BreakTransform` (`self.GetTransform` (`self.Random Spawn`))))
  (bind (_returnvalue_location_3 _returnvalue_rotation_3) (`KismetMathLibrary.BreakTransform` (`self.GetTransform` (`self.Random Spawn`))))
  (bind (_returnvalue_location_4 _returnvalue_rotation_4) (`KismetMathLibrary.BreakTransform` (`self.GetTransform` (`self.Random Spawn`))))
  (bind (_returnvalue_location_5 _returnvalue_rotation_5) (`KismetMathLibrary.BreakTransform` (`self.GetTransform` (`self.Random Spawn`))))
  (bind (_returnvalue_location_6 _returnvalue_rotation_6) (`KismetMathLibrary.BreakTransform` (`self.GetTransform` (`self.Random Spawn`))))
  (bind (_returnvalue_location_7 _returnvalue_rotation_7) (`KismetMathLibrary.BreakTransform` (`self.GetTransform` (`self.Random Spawn`))))
  (bind (_returnvalue_location_8 _returnvalue_rotation_8) (`KismetMathLibrary.BreakTransform` (`self.GetTransform` (`self.Random Spawn`))))
  (if (`self.Tuto Finish?`)
    (set `self.Timer` (+ (`self.Timer`) 1))
    (if (!= (`self.Time spawn`) 0.5)
      (set `self.Time spawn` (- (`self.Time spawn`) 0.005)))
    (set `self.rd` (`KismetMathLibrary.RandomIntegerInRange` 1 3))
    (if (== (`self.rd`) 3)
      (`AIBlueprintHelperLibrary.SpawnAIFromClass` "/Game/Valentin/BluePrint/Ennemie/BP_FusilsBritish.BP_FusilsBritish_C" null _returnvalue_location_3 _returnvalue_rotation_3 false null)
      (else
        (`AIBlueprintHelperLibrary.SpawnAIFromClass` "/Game/Valentin/BluePrint/Ennemie/BP_Fantassin.BP_Fantassin_C" null _returnvalue_location_2 _returnvalue_rotation_2 false null)))
    (set `self.rd` (`KismetMathLibrary.RandomIntegerInRange` 1 3))
    (if (== (`self.rd`) 3)
      (`AIBlueprintHelperLibrary.SpawnAIFromClass` "/Game/Valentin/BluePrint/Ennemie/BP_FusilsBritish.BP_FusilsBritish_C" null _returnvalue_location_5 _returnvalue_rotation_5 false null)
      (else
        (`AIBlueprintHelperLibrary.SpawnAIFromClass` "/Game/Valentin/BluePrint/Ennemie/BP_Fantassin.BP_Fantassin_C" null _returnvalue_location_4 _returnvalue_rotation_4 false null)))
    (if (>= (`self.Timer`) 20)
      (set `self.rd` (`KismetMathLibrary.RandomIntegerInRange` 1 3))
      (if (== (`self.rd`) 3)
        (`AIBlueprintHelperLibrary.SpawnAIFromClass` "/Game/Valentin/BluePrint/Ennemie/BP_FusilsBritish.BP_FusilsBritish_C" null _returnvalue_location_7 _returnvalue_rotation_7 false null)
        (else
          (`AIBlueprintHelperLibrary.SpawnAIFromClass` "/Game/Valentin/BluePrint/Ennemie/BP_Fantassin.BP_Fantassin_C" null _returnvalue_location_6 _returnvalue_rotation_6 false null)))
      (if (>= (`self.Timer`) 35)
        (set `self.rd` (`KismetMathLibrary.RandomIntegerInRange` 1 3))
        (if (== (`self.rd`) 3)
          (`AIBlueprintHelperLibrary.SpawnAIFromClass` "/Game/Valentin/BluePrint/Ennemie/BP_FusilsBritish.BP_FusilsBritish_C" null _returnvalue_location_8 _returnvalue_rotation_8 false null)
          (else
            (`AIBlueprintHelperLibrary.SpawnAIFromClass` "/Game/Valentin/BluePrint/Ennemie/BP_Fantassin.BP_Fantassin_C" null _returnvalue_location _returnvalue_rotation false null)))))))

(fn `Random Enemy`
  (set `self.rd` (`KismetMathLibrary.RandomIntegerInRange` 1 3))
  (if (== (`self.rd`) 3)
    _))

(fn `Random Spawn`
  (returns (OutItem :type "/Game/Valentin/BluePrint/Spawn/BP_SpawnPoint Object Reference"))
  (return (`KismetArrayLibrary.Array_Random` (`self.Spawn Point`))))

(fn `UserConstructionScript`)