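; BP_IndChaman is a tower Blueprint, apparently the Indian shaman variant, that fires phantom projectiles for the non-French side.
; On BeginPlay it calls its parent, then sets the faction flag, projectile class, fire delay and upgrade price, leaving overlap handling to the parent.
; Every Tick it runs LevelModifieur, which reapplies the tower mesh matching Level 2 or 3 rather than swapping it only on upgrade.
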(event `self.ReceiveBeginPlay`
  (`parent.ReceiveBeginPlay`)
  (set `self.I'm french?` false)
  (set `self.Amo Type` "/Game/Valentin/BluePrint/projectile/Allier/Chaman/BP_PhantomeProj.BP_PhantomeProj_C")
  (set `self.Time to Shoot` 0.7)
  (set `self.Prix amélioration` 12))

(event `self.ReceiveActorBeginOverlap`
  (params (OtherActor :type "Actor Object Reference"))
  (`parent.ReceiveActorBeginOverlap` OtherActor))

(event `self.ReceiveTick`
  (params (DeltaSeconds :type "Float (single-precision)"))
  (`parent.ReceiveTick` DeltaSeconds)
  (`self.Level Modifieur`))

(event `Level Modifieur`
  (if (== (`self.Level`) 2)
    (`StaticMeshComponent.SetStaticMesh` (`self.Tower`) "/Game/Asset3d/Tour_Indiens/TOWI_LV2_MESH.TOWI_LV2_MESH")
    (elif (== (`self.Level`) 3)
      (`StaticMeshComponent.SetStaticMesh` (`self.Tower`) "/Game/Asset3d/Tour_Indiens/TOWI_LV3_MESH.TOWI_LV3_MESH"))))

(fn `UserConstructionScript`
  (`parent.UserConstructionScript`))