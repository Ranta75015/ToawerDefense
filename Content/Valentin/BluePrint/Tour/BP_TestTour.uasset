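; BP_TestTour is a defense tower that tracks and shoots BP_TestEnemie actors, takes damage and destroys itself at zero life.
; While active, overlaps fill a target list and register the tower on each enemy; exits unregister it.
; Tick rotates Corp toward the first target and spawns ammo at Mire, paced by a Delay.
; Tick also refreshes the health bar widget and raises the tower while the mouse hovers its slot.
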(event `self.ReceiveBeginPlay`
  (set `self.Pos de Base` (`self.K2_GetActorLocation`))
  (set `self.What I move to shoot` (`self.Corp`))
  (set `self.Amo Type` "/Game/Valentin/BluePrint/projectile/Allier/BP_Amo.BP_Amo_C"))

(event `self.ReceiveActorEndOverlap`
  (params (OtherActor :type "Actor Object Reference"))
  (bind _asbp_test_enemie (cast `/Game/Valentin/BluePrint/BP_TestEnemie` OtherActor))
  (`KismetArrayLibrary.Array_RemoveItem` (`self.Liste ennemie`) _asbp_test_enemie)
  (set `/Game/Valentin/BluePrint/BP_TestEnemie.I'm Lock By Tower?` true _asbp_test_enemie)
  (`KismetArrayLibrary.Array_RemoveItem` (`/Game/Valentin/BluePrint/BP_TestEnemie.Tower Lock` _asbp_test_enemie) self))

(event `Updaet life`
  (params (DeltaSeconds :type "Float (single-precision)"))
  (bind _life (`self.Life`))
  ;[0 1 0.2406] Mise a jour vie
  (bind _asui_life_friends (cast `/Game/Valentin/Ui/UI_LifeFriends` (`WidgetComponent.GetWidget` (`self.Life Bar`))))
  (`/Game/Valentin/Ui/UI_LifeFriends.Update Health bar` _asui_life_friends _life (`self.MinLife`) (`self.MaxLife`))
  (if (<= _life 0.0)
    (`self.K2_DestroyActor`)))

(event `Feed Back Souri`
  (bind _my_slot (`self.My Slot`))
  ;[1 0.9385 0] Feed Back si la souris survole
  (`/Engine/EditorBlueprintResources/StandardMacros.IsValid` _my_slot
    (:`Is Valid`
      (if (`/Game/Valentin/BluePrint/BP_SlotBordChemin.Is over?` _my_slot)
        (`self.K2_SetActorLocation` (+ (`self.Pos de Base`) (* (`self.GetActorUpVector`) (`self.Up`))))
        (else
          (`self.K2_SetActorLocation` (`self.Pos de Base`)))))))

(event `self.ReceiveActorBeginOverlap`
  (params (OtherActor :type "Actor Object Reference"))
  (if (`self.I'm active?`)
    (bind _asbp_test_enemie (cast `/Game/Valentin/BluePrint/BP_TestEnemie` OtherActor))
    (`KismetArrayLibrary.Array_Add` (`self.Liste ennemie`) _asbp_test_enemie)
    (set `/Game/Valentin/BluePrint/BP_TestEnemie.I'm Lock By Tower?` true _asbp_test_enemie)
    (`KismetArrayLibrary.Array_Add` (`/Game/Valentin/BluePrint/BP_TestEnemie.Tower Lock` _asbp_test_enemie) self)))

(event `self.ReceiveTick`
  (params (DeltaSeconds :type "Float (single-precision)"))
  (bind _liste_ennemie (`self.Liste ennemie`))
  (`self.Feed Back Souri`)
  (`self.Updaet life` 0.0)
  (`self.Folow targert`)
  (`self.fire`)
  (`/Engine/EditorBlueprintResources/StandardMacros.IsValid` (`|GetArrayItem` _liste_ennemie)
    (:`Is Not Valid`
      (`KismetArrayLibrary.Array_Remove` _liste_ennemie))))

(event `fire`
  (if (not (`KismetArrayLibrary.Array_IsEmpty` (`self.Liste ennemie`)))
    (`KismetSystemLibrary.Delay` (`self.Time to Shoot`))
    (`|SpawnActorFromClass` (`self.Amo Type`) (`SceneComponent.K2_GetComponentToWorld` (`self.Mire`)) "Undefined" "OverrideRootScale" null null)))

(event `self.ReceiveAnyDamage`
  (params (Damage :type "Float (single-precision)") (DamageType :type "DamageType Object Reference") (InstigatedBy :type "Controller Object Reference") (DamageCauser :type "Actor Object Reference"))
  (set `self.Life` (- (`self.Life`) Damage)))

(fn `Folow targert`
  (bind (_returnvalue_roll _returnvalue_pitch _returnvalue_yaw) (`KismetMathLibrary.BreakRotator` (`KismetMathLibrary.FindLookAtRotation` (`SceneComponent.K2_GetComponentLocation` (`self.Corp`)) (`self.K2_GetActorLocation` (`|GetArrayItem` (`self.Liste ennemie`))))))
  (`/Engine/EditorBlueprintResources/StandardMacros.IsValid` (`|GetArrayItem` (`self.Liste ennemie`))
    (:`Is Valid`
      (`SceneComponent.K2_SetRelativeRotation` (`self.Corp`) (`KismetMathLibrary.MakeRotator` 0.0 _returnvalue_pitch _returnvalue_yaw) false false))))

(fn `UserConstructionScript`)