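; BP_FrCanon is the French cannon tower, a child Blueprint that specialises a parent tower class.
; On BeginPlay it runs the parent logic, then sets its fire timing, BP_bouler ammo type, French faction flag and upgrade price.
; Every Tick it calls LevelModifieur, which swaps the visible tower component to match Level 2 or 3 by toggling hidden-in-game on the Tower components.
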(event `self.ReceiveBeginPlay`
  (`parent.ReceiveBeginPlay`)
  (set `self.Time to Shoot` 2.0)
  (set `self.Amo Type` "/Game/Valentin/BluePrint/projectile/Allier/Bouler/BP_bouler.BP_bouler_C")
  (set `self.I'm french?` true)
  (set `self.Prix amélioration` 18))

(event `self.ReceiveActorBeginOverlap`
  (params (OtherActor :type "Actor Object Reference"))
  (`parent.ReceiveActorBeginOverlap` OtherActor))

(event `self.ReceiveTick`
  (params (DeltaSeconds :type "Float (single-precision)"))
  (`parent.ReceiveTick` DeltaSeconds)
  (`self.Level Modifieur`))

(event `Level Modifieur`
  (if (== (`self.Level`) 2)
    (`SceneComponent.SetHiddenInGame` (`self.Tower 2`) false false)
    (`SceneComponent.SetHiddenInGame` (`self.Tower 1`) true false)
    (elif (== (`self.Level`) 3)
      (`SceneComponent.SetHiddenInGame` (`self.Tower 3`) false false)
      (`SceneComponent.SetHiddenInGame` (`self.Tower 2`) true false))))

(fn `UserConstructionScript`
  (`parent.UserConstructionScript`))