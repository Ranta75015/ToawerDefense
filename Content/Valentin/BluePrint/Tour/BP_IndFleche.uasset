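; BP_IndFleche is an arrow tower for the non-French side, built as a child of a parent tower Blueprint.
; BeginPlay calls the parent, then sets the fire delay, BP_fleche as the ammo type and clears the ImFrench flag.
; Every tick it runs the parent logic, then LevelModifieur, which reapplies the matching Tower static mesh while Level is two or three.
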(event `self.ReceiveBeginPlay`
  (`parent.ReceiveBeginPlay`)
  (set `self.Time to Shoot` 0.6)
  (set `self.Amo Type` "/Game/Valentin/BluePrint/projectile/Allier/BP_fleche.BP_fleche_C")
  (set `self.I'm french?` false))

(event `self.ReceiveActorBeginOverlap`
  (params (OtherActor :type "Actor Object Reference"))
  (`parent.ReceiveActorBeginOverlap` OtherActor))

(event `self.ReceiveTick`
  (params (DeltaSeconds :type "Float (single-precision)"))
  (`parent.ReceiveTick` DeltaSeconds)
  (`self.Level Modifieur`))

(event `Level Modifieur`
  (if (== (`self.Level`) 2)
    (`StaticMeshComponent.SetStaticMesh` (`self.Tower`) "/Game/Asset3d/Tour_Indiens/TOWI_LV2_MESH.TOWI_LV2_MESH")
    (elif (== (`self.Level`) 3)
      (`StaticMeshComponent.SetStaticMesh` (`self.Tower`) "/Game/Asset3d/Tour_Indiens/TOWI_LV3_MESH.TOWI_LV3_MESH"))))

(fn `UserConstructionScript`
  (`parent.UserConstructionScript`))