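; BP_FrFusil is a French rifle tower, a child Blueprint that configures its parent tower class.
; On BeginPlay it sets the fire delay, BP_Amo ammo type, French side flag and upgrade price after the parent logic runs.
; Every Tick it calls LevelModifieur, which swaps the visible Tower component for levels 2 and 3 by polling Level rather than reacting to upgrades.
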(event `self.ReceiveBeginPlay`
  (`parent.ReceiveBeginPlay`)
  (set `self.Time to Shoot` 0.8)
  (set `self.Amo Type` "/Game/Valentin/BluePrint/projectile/Allier/BP_Amo.BP_Amo_C")
  (set `self.I'm french?` true)
  (set `self.Prix amélioration` 12))

(event `self.ReceiveActorBeginOverlap`
  (params (OtherActor :type "Actor Object Reference"))
  (`parent.ReceiveActorBeginOverlap` OtherActor))

(event `self.ReceiveTick`
  (params (DeltaSeconds :type "Float (single-precision)"))
  (`parent.ReceiveTick` DeltaSeconds)
  (`self.Level Modifieur`))

(event `Level Modifieur`
  (if (== (`self.Level`) 2)
    (`SceneComponent.SetHiddenInGame` (`self.Tower 2`) false false)
    (`SceneComponent.SetHiddenInGame` (`self.Tower 1`) true false)
    (elif (== (`self.Level`) 3)
      (`SceneComponent.SetHiddenInGame` (`self.Tower 3`) false false)
      (`SceneComponent.SetHiddenInGame` (`self.Tower 2`) true false))))

(fn `UserConstructionScript`
  (`parent.UserConstructionScript`))