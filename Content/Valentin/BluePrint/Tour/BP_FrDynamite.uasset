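; BP_FrDynamite is a French dynamite tower that inherits its core behavior from a parent Blueprint.
; On BeginPlay it sets the fire delay, uses BP_DynamiteP as its ammo type and flags itself as French.
; Every Tick, after the parent logic, it checks Level and swaps the visible tower component at levels 2 and 3.
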(event `self.ReceiveBeginPlay`
  (`parent.ReceiveBeginPlay`)
  (set `self.Time to Shoot` 1.0)
  (set `self.Amo Type` "/Game/Valentin/BluePrint/projectile/Allier/Dynamite/BP_DynamiteP.BP_DynamiteP_C")
  (set `self.I'm french?` true))

(event `self.ReceiveActorBeginOverlap`
  (params (OtherActor :type "Actor Object Reference"))
  (`parent.ReceiveActorBeginOverlap` OtherActor))

(event `self.ReceiveTick`
  (params (DeltaSeconds :type "Float (single-precision)"))
  (`parent.ReceiveTick` DeltaSeconds)
  (`self.Level Modifieur`))

(event `Level Modifieur`
  (if (== (`self.Level`) 2)
    (`SceneComponent.SetHiddenInGame` (`self.Tower 2`) false false)
    (`SceneComponent.SetHiddenInGame` (`self.Tower 1`) true false)
    (elif (== (`self.Level`) 3)
      (`SceneComponent.SetHiddenInGame` (`self.Tower 3`) false false)
      (`SceneComponent.SetHiddenInGame` (`self.Tower 2`) true false))))

(fn `UserConstructionScript`
  (`parent.UserConstructionScript`))