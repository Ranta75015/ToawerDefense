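; Player pawn Blueprint that handles directional movement and mouse-wheel camera zoom.
; Forward/backward and right/left input axes feed movement input along the actor's own forward and right vectors.
; The mouse wheel changes the SpringArm length in fixed steps, gated by MaxZoom and MaxDezoom limits checked before each step.
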(event `Key|MouseScrollDown`
  (params (Key :type "Key Structure"))
  (bind _springarm (`self.SpringArm`))
  (bind _targetarmlength (`SpringArmComponent.TargetArmLength` _springarm))
  ;[1 0.1645 0.9183] Camera Role
  (:`Pressed`
    (if (not (>= _targetarmlength (`self.Max dezoom`)))
      (set `SpringArmComponent.TargetArmLength` (+ 20.0 _targetarmlength) _springarm))))

(event `InputAxis|Move Forward / Backward`
  (params (AxisValue :type "Float (single-precision)"))
  ;[0.07743 1 0.9003] Mouvment
  (`self.AddMovementInput` (`self.GetActorForwardVector`) AxisValue))

(event `InputAxis|Move Right / Left`
  (params (AxisValue :type "Float (single-precision)"))
  ;[0.07743 1 0.9003] Mouvment
  (`self.AddMovementInput` (`self.GetActorRightVector`) AxisValue))

(event `Key|MouseScrollUp`
  (params (Key :type "Key Structure"))
  (bind _springarm (`self.SpringArm`))
  (bind _targetarmlength (`SpringArmComponent.TargetArmLength` _springarm))
  ;[1 0.1645 0.9183] Camera Role
  (:`Pressed`
    (if (not (<= _targetarmlength (`self.Max zoom`)))
      (set `SpringArmComponent.TargetArmLength` (- _targetarmlength 20.0) _springarm))))

(fn `UserConstructionScript`)