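; Spike trap that periodically damages every enemy in its ListeEnnemie list and wears down over time.
; On BeginPlay it flags itself as a spike and starts two looping timers.
; The damage timer toggles ON and applies damage only when switching on, so hits land on alternate ticks.
; The AutoDestroy timer only lowers Life; overlap and Tick just call the parent.
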(event `auto destroy`
  (set `self.Life` (- (`self.Life`) 5.0)))

(event `self.ReceiveBeginPlay`
  (`parent.ReceiveBeginPlay`)
  (set `self.I'm Spike?` true)
  (`KismetSystemLibrary.K2_SetTimerDelegate` (delegate `deal damage`) 2.5 true)
  (`KismetSystemLibrary.K2_SetTimerDelegate` (delegate `auto destroy`) 10.0 true))

(event `deal damage`
  (bind _liste_ennemie (`self.Liste ennemie`))
  (if (`self.ON?`)
    (set `self.ON?` false)
    (else
      (set `self.ON?` true)
      (for (_ _array_index) _liste_ennemie
        (`GameplayStatics.ApplyDamage` (`|GetArrayItem` _liste_ennemie _array_index) 3.0)))))

(event `self.ReceiveActorBeginOverlap`
  (params (OtherActor :type "Actor Object Reference"))
  (`parent.ReceiveActorBeginOverlap` OtherActor))

(event `self.ReceiveTick`
  (params (DeltaSeconds :type "Float (single-precision)"))
  (`parent.ReceiveTick` DeltaSeconds))

(fn `UserConstructionScript`
  (`parent.UserConstructionScript`))