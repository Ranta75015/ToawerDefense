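; BP_ShootWall is a trap wall with health that tracks overlapping BP_TestEnemie actors and can damage them.
; Overlap flags enemies as blocked, unless the trap is a bomb or spike, and registers the wall with them.
; Tick refreshes the health bar, destroys the wall at zero life, prunes invalid enemies and raises it while its slot is hovered.
; The fire event, not called here, damages the first listed enemy after a delay.
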(event `Update life`
  (bind _life (`self.Life`))
  ;[0 1 0.2406] Mise a jour vie
  (bind _asui_life_friends (cast `/Game/Valentin/Ui/UI_LifeFriends` (`WidgetComponent.GetWidget` (`self.Life Bar`))))
  (`/Game/Valentin/Ui/UI_LifeFriends.Update Health bar` _asui_life_friends _life (`self.MinLife`) (`self.MaxLife`))
  (if (<= _life 0.0)
    (`self.K2_DestroyActor`)))

(event `self.ReceiveActorEndOverlap`
  (params (OtherActor :type "Actor Object Reference"))
  (bind _asbp_test_enemie (cast `/Game/Valentin/BluePrint/Ennemie/BP_TestEnemie` OtherActor))
  (`KismetArrayLibrary.Array_RemoveItem` (`self.Liste ennemie`) _asbp_test_enemie)
  (set `/Game/Valentin/BluePrint/Ennemie/BP_TestEnemie.I have Wall Front?` false _asbp_test_enemie)
  (`KismetArrayLibrary.Array_RemoveItem` (`/Game/Valentin/BluePrint/Ennemie/BP_TestEnemie.Wall Lock` _asbp_test_enemie) self))

(event `Feed Back Souri`
  (bind _my_slot (`self.My Slot`))
  ;[1 0.9385 0] Feed Back si la souris survole
  (`/Engine/EditorBlueprintResources/StandardMacros.IsValid` _my_slot
    (:`Is Valid`
      (if (`/Game/Valentin/BluePrint/BP_SlotChemin.Is over?` _my_slot)
        (`self.K2_SetActorLocation` (+ (`self.Pos de Base`) (* (`self.GetActorUpVector`) (`self.Up`))))
        (else
          (`self.K2_SetActorLocation` (`self.Pos de Base`)))))))

(event `self.ReceiveActorBeginOverlap`
  (params (OtherActor :type "Actor Object Reference"))
  (bind _asbp_test_enemie (cast `/Game/Valentin/BluePrint/Ennemie/BP_TestEnemie` OtherActor))
  (`KismetArrayLibrary.Array_Add` (`self.Liste ennemie`) _asbp_test_enemie)
  (if (`self.I'm a Bombe?`)
    _
    (elif (not (`self.I'm Spike?`))
      (set `/Game/Valentin/BluePrint/Ennemie/BP_TestEnemie.I have Wall Front?` true _asbp_test_enemie)
      (if (`/Game/Valentin/BluePrint/Ennemie/BP_TestEnemie.I have Wall Front?` _asbp_test_enemie)
        (`KismetArrayLibrary.Array_Add` (`/Game/Valentin/BluePrint/Ennemie/BP_TestEnemie.Wall Lock` _asbp_test_enemie) self)))))

(event `self.ReceiveAnyDamage`
  (params (Damage :type "Float (single-precision)") (DamageType :type "DamageType Object Reference") (InstigatedBy :type "Controller Object Reference") (DamageCauser :type "Actor Object Reference"))
  (set `self.Life` (- (`self.Life`) Damage)))

(event `self.ReceiveBeginPlay`
  (set `self.Pos de Base` (`self.K2_GetActorLocation`)))

(event `self.ReceiveTick`
  (params (DeltaSeconds :type "Float (single-precision)"))
  (bind _liste_ennemie (`self.Liste ennemie`))
  (`self.Feed Back Souri`)
  (`self.Update life`)
  (`/Engine/EditorBlueprintResources/StandardMacros.IsValid` (`|GetArrayItem` _liste_ennemie)
    (:`Is Not Valid`
      (`KismetArrayLibrary.Array_Remove` _liste_ennemie))))

(event `fire`
  (bind _liste_ennemie (`self.Liste ennemie`))
  (if (not (`KismetArrayLibrary.Array_IsEmpty` _liste_ennemie))
    (`KismetSystemLibrary.Delay` 0.3)
    (`GameplayStatics.ApplyDamage` (`|GetArrayItem` _liste_ennemie) 1.0)))

(fn `UserConstructionScript`)