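; Test enemy character that marches toward a fort location and shoots at towers, blocking walls or the fort.
; A looping timer drops invalid locks, then prioritises a locked tower over a front wall, turning toward it and spawning projectiles, or fires at the fort when facing it.
; Rain totem walls are not targeted but slow its walk speed.
; Tick updates the health bar widget and destroys the actor shortly after life runs out.
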(event `self.ReceiveAnyDamage`
  (params (Damage :type "Float (single-precision)") (DamageType :type "DamageType Object Reference") (InstigatedBy :type "Controller Object Reference") (DamageCauser :type "Actor Object Reference"))
  (set `self.Life` (- (`self.Life`) Damage)))

(event `Ralentir`
  (bind _charactermovement (`self.CharacterMovement`))
  (if (`self.I have Wall Front?`)
    (if (== (`GameplayStatics.GetObjectClass` (`|GetArrayItem` (`self.Wall Lock`))) "/Game/Valentin/BluePrint/Trap/BP_TotemPluie.BP_TotemPluie_C")
      (set `CharacterMovementComponent.MaxWalkSpeed` (`self.Walk lent`) _charactermovement))
    (else
      (set `CharacterMovementComponent.MaxWalkSpeed` 300.0 _charactermovement))))

(event `self.ReceiveTick`
  (params (DeltaSeconds :type "Float (single-precision)"))
  (bind _life (`self.Life`))
  ;[0 1 0.2406] Mise a jour vie
  (bind _asui_life_ennemies (cast `/Game/Valentin/Ui/UI_LifeEnnemies` (`WidgetComponent.GetWidget` (`self.LifePoint`))))
  (`/Game/Valentin/Ui/UI_LifeEnnemies.Update Health bar` _asui_life_ennemies _life (`self.MinLife`) (`self.MaxLife`))
  (`self.Ralentir`)
  (if (<= _life 0.0)
    (set `self.I'm dead?` true)
    (`KismetSystemLibrary.Delay` 1.2)
    (`self.K2_DestroyActor`)))

(event `Move`
  ;[0.3032 0.1758 1] IA Mouvment
  (`AIBlueprintHelperLibrary.SimpleMoveToLocation` (`AIBlueprintHelperLibrary.GetAIController` self) (`self.Target`)))

(event `self.ReceiveBeginPlay`
  ;[0.3032 0.1758 1] IA Mouvment
  (if (not (`self.I'm dead?`))
    (set `self.Target` (`self.Loaclisation Fort`))
    (`self.Move`)
    (`KismetSystemLibrary.K2_SetTimerDelegate` (delegate `Update target`) (`self.Time to shoot`) true)))

(event `Update target`
  (bind _tower_lock (`self.Tower Lock`))
  (bind _wall_lock (`self.Wall Lock`))
  (bind _capsulecomponent (`self.CapsuleComponent`))
  (bind _capsulecomponent_2 (`self.CapsuleComponent`))
  (bind _output (`|GetArrayItem` _tower_lock))
  (bind _output_2 (`|GetArrayItem` _wall_lock))
  (bind (_returnvalue_roll _returnvalue_pitch _returnvalue_yaw) (`KismetMathLibrary.BreakRotator` (`KismetMathLibrary.FindLookAtRotation` (`SceneComponent.K2_GetComponentLocation` _capsulecomponent_2) (`self.K2_GetActorLocation` _output_2))))
  (bind (_returnvalue_roll_2 _returnvalue_pitch_2 _returnvalue_yaw_2) (`KismetMathLibrary.BreakRotator` (`KismetMathLibrary.FindLookAtRotation` (`SceneComponent.K2_GetComponentLocation` _capsulecomponent) (`self.K2_GetActorLocation` _output))))
  ;[0.3032 0.1758 1] IA Mouvment
  (if (not (`self.I'm dead?`))
    (`/Engine/EditorBlueprintResources/StandardMacros.IsValid` _output
      (:`Is Valid`
        _)
      (:`Is Not Valid`
        (`KismetArrayLibrary.Array_Remove` _tower_lock)
        (set `self.I'm Lock By Tower?` false)))
    (`/Engine/EditorBlueprintResources/StandardMacros.IsValid` _output_2
      (:`Is Valid`
        _)
      (:`Is Not Valid`
        (`KismetArrayLibrary.Array_Remove` _wall_lock)
        (set `self.I have Wall Front?` false)))
    (if (`self.I'm Lock By Tower?`)
      (if (not (`self.I shoot?`))
        (`KismetSystemLibrary.Delay` (`KismetMathLibrary.RandomFloatInRange` 0.3 1.0))
        (set `self.I shoot?` true))
      (set `self.Target` (`self.K2_GetActorLocation` _output))
      (`SceneComponent.K2_SetRelativeRotation` _capsulecomponent (`KismetMathLibrary.MakeRotator` 0.0 0.0 _returnvalue_yaw_2) false false)
      (`|SpawnActorFromClass` (`self.Amo`) (`SceneComponent.K2_GetComponentToWorld` (`self.mire`)) "Undefined" "OverrideRootScale" null null)
      (`self.Move` :!label _label)
      (else
        (set `self.I shoot?` false)
        (if (`self.I have Wall Front?`)
          (if (== (`GameplayStatics.GetObjectClass` (`|GetArrayItem` (`self.Wall Lock`))) "/Game/Valentin/BluePrint/Trap/BP_TotemPluie.BP_TotemPluie_C")
            _
            (else
              (set `self.Target` (`self.K2_GetActorLocation` _output_2))
              (`SceneComponent.K2_SetRelativeRotation` _capsulecomponent_2 (`KismetMathLibrary.MakeRotator` 0.0 0.0 _returnvalue_yaw) false false)
              (`|SpawnActorFromClass` (`self.Amo`) (`SceneComponent.K2_GetComponentToWorld` (`self.mire`)) "Undefined" "OverrideRootScale" null null)
              (set `self.Shoot on Wall?` true)
              (goto _label)))
          (else
            (set `self.Shoot on Wall?` false)))
        (if (`self.I'm Face TO Fort?`)
          (if (not (`self.Wait For Shot`))
            (`KismetSystemLibrary.Delay` (`KismetMathLibrary.RandomFloatInRange` 0.2 1.0))
            (`MovementComponent.StopMovementImmediately` (`self.CharacterMovement`))
            (set `self.Wait For Shot` true))
          (`|SpawnActorFromClass` (`self.Amo`) (`SceneComponent.K2_GetComponentToWorld` (`self.mire`)) "Undefined" "OverrideRootScale" null null)
          (set `self.I shoot?` true)
          (else
            (set `self.Target` (`self.Loaclisation Fort`))
            (goto _label)))))))

(fn `UserConstructionScript`)