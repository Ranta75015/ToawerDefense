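; BP_TestDéfense is a test Blueprint for a damageable object that displays its health on a LifeBar widget.
; AnyDamage subtracts incoming damage from Life, with no clamping or death handling in the graph.
; Every Tick, it casts the LifeBar widget to UI_LifeFriends and pushes Life with its min and max range to UpdateHealthBar, polling rather than updating on damage.
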(event `self.ReceiveTick`
  (params (DeltaSeconds :type "Float (single-precision)"))
  ;[0 1 0.2406] Mise a jour vie
  (bind _asui_life_friends (cast `/Game/Valentin/Ui/UI_LifeFriends` (`WidgetComponent.GetWidget` (`self.LifeBar`))))
  (`/Game/Valentin/Ui/UI_LifeFriends.Update Health bar` _asui_life_friends (`self.Life`) (`self.MinLife`) (`self.MaxLife`)))

(event `self.ReceiveAnyDamage`
  (params (Damage :type "Float (single-precision)") (DamageType :type "DamageType Object Reference") (InstigatedBy :type "Controller Object Reference") (DamageCauser :type "Actor Object Reference"))
  (set `self.Life` (- (`self.Life`) Damage)))

(fn `UserConstructionScript`)