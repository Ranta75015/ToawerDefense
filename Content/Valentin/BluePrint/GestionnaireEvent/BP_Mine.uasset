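; BP_Mine is a mine actor that periodically adds gold to BP_FinalPlayer and raises random events.
; A looping timer shows its widget and opens a timed window; if still unresolved afterward, all three player mood values drop.
; Releasing a click on the cube rolls a weighted random event panel, passing the mine to it.
; The Espritenerves range check is contradictory, so that event never fires.
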(event `self.ReceiveBeginPlay`
  (`KismetSystemLibrary.K2_SetTimerDelegate` (delegate `PoP event`) 1.0 true)
  (`KismetSystemLibrary.K2_SetTimerDelegate` (delegate `Add Gold`) 5.0 true))

(event `PoP event`
  (if (not (`self.Event is on?`))
    (set `self.Event is on?` true)
    (set `self.reolve?` false)
    (`SceneComponent.SetHiddenInGame` (`self.Widget`) false false)
    (`KismetSystemLibrary.Delay` 30.0)
    (if (`self.reolve?`)
      (set `self.Event is on?` false)
      (set `self.is clicked?` false)
      (else
        (set `self.Event is on?` false)
        (`SceneComponent.SetHiddenInGame` (`self.Widget`) true false)
        (bind _asbp_final_player (cast `/Game/Valentin/BluePrint/BP_FinalPlayer` (`GameplayStatics.GetPlayerPawn` 0)))
        (set `/Game/Valentin/BluePrint/BP_FinalPlayer.Humeur Phan` (- (`/Game/Valentin/BluePrint/BP_FinalPlayer.Humeur Phan` _asbp_final_player) 5) _asbp_final_player)
        (set `/Game/Valentin/BluePrint/BP_FinalPlayer.Humeur Ind` (- (`/Game/Valentin/BluePrint/BP_FinalPlayer.Humeur Ind` _asbp_final_player) 5) _asbp_final_player)
        (set `/Game/Valentin/BluePrint/BP_FinalPlayer.Humeur Fr` (- (`/Game/Valentin/BluePrint/BP_FinalPlayer.Humeur Fr` _asbp_final_player) 5) _asbp_final_player)
        (set `self.is clicked?` false)))))

(event `Add Gold`
  (bind _asbp_final_player (cast `/Game/Valentin/BluePrint/BP_FinalPlayer` (`GameplayStatics.GetPlayerPawn` 0)))
  (set `/Game/Valentin/BluePrint/BP_FinalPlayer.Gold` (+ (`/Game/Valentin/BluePrint/BP_FinalPlayer.Gold` _asbp_final_player) (+ (`self.Bonus Gold`) 1 (`self.Bonus humeur`))) _asbp_final_player))

(event `self.Cube.OnReleased`
  (params (TouchedComponent :type "PrimitiveComponent Object Reference") (ButtonReleased :type "Key Structure"))
  (if (not (`self.is clicked?`))
    (set `self.is clicked?` true)
    (`SceneComponent.SetHiddenInGame` (`self.Widget`) true false)
    (set `self.num event` (`KismetMathLibrary.RandomIntegerInRange` 0 100))
    (if (and (<= (`self.num event`) 100) (>= (`self.num event`) 96))
      (bind _returnvalue (`|CreateWidget` "/Game/Mathis/UI/UI_Event_Amelioration.UI_Event_Amelioration_C"))
      (set `/Game/Mathis/UI/UI_Event_Amelioration.Mine` self _returnvalue)
      (`UserWidget.AddToViewport` _returnvalue 0)
      (`|PlayAnimationTimeRange` _returnvalue (`/Game/Mathis/UI/UI_Event_Amelioration.Slide_Panel_Amélioration` _returnvalue))
      (elif (and (<= (`self.num event`) 95) (>= (`self.num event`) 91))
        (bind _returnvalue_2 (`|CreateWidget` "/Game/Mathis/UI/UI_Event_Entretien.UI_Event_Entretien_C"))
        (set `/Game/Mathis/UI/UI_Event_Entretien.Mine` self _returnvalue_2)
        (`UserWidget.AddToViewport` _returnvalue_2 0)
        (`|PlayAnimationTimeRange` _returnvalue_2 (`/Game/Mathis/UI/UI_Event_Entretien.Slide_Panel_Entretien` _returnvalue_2))
        (elif (and (<= (`self.num event`) 0) (>= (`self.num event`) 15))
          (bind _returnvalue_3 (`|CreateWidget` "/Game/Mathis/UI/UI_Event_Espritenerves.UI_Event_Espritenerves_C"))
          (set `/Game/Mathis/UI/UI_Event_Espritenerves.Mine` self _returnvalue_3)
          (`UserWidget.AddToViewport` _returnvalue_3 0)
          (`|PlayAnimationTimeRange` _returnvalue_3 (`/Game/Mathis/UI/UI_Event_Espritenerves.Slide_Panel_Espritsénervés` _returnvalue_3))
          (elif (and (<= (`self.num event`) 30) (>= (`self.num event`) 26))
            (bind _returnvalue_4 (`|CreateWidget` "/Game/Mathis/UI/UI_Event_fete.UI_Event_fete_C"))
            (set `/Game/Mathis/UI/UI_Event_fete.Mine` self _returnvalue_4)
            (`UserWidget.AddToViewport` _returnvalue_4 0)
            (`|PlayAnimationTimeRange` _returnvalue_4 (`/Game/Mathis/UI/UI_Event_fete.Slide_Panel_Fête` _returnvalue_4))
            (elif (and (<= (`self.num event`) 90) (>= (`self.num event`) 86))
              (bind _returnvalue_5 (`|CreateWidget` "/Game/Mathis/UI/UI_Event_HymneNational.UI_Event_HymneNational_C"))
              (set `/Game/Mathis/UI/UI_Event_HymneNational.Mine` self _returnvalue_5)
              (`UserWidget.AddToViewport` _returnvalue_5 0)
              (`|PlayAnimationTimeRange` _returnvalue_5 (`/Game/Mathis/UI/UI_Event_HymneNational.Slide_Panel_HymneNational` _returnvalue_5))
              (elif (and (<= (`self.num event`) 85) (>= (`self.num event`) 66))
                (bind _returnvalue_6 (`|CreateWidget` "/Game/Mathis/UI/UI_Event_offrande.UI_Event_offrande_C"))
                (set `/Game/Mathis/UI/UI_Event_offrande.Mine` self _returnvalue_6)
                (`UserWidget.AddToViewport` _returnvalue_6 0)
                (`|PlayAnimationTimeRange` _returnvalue_6 (`/Game/Mathis/UI/UI_Event_offrande.Slide_Panel_Offrande` _returnvalue_6))
                (elif (and (<= (`self.num event`) 25) (>= (`self.num event`) 16))
                  (bind _returnvalue_7 (`|CreateWidget` "/Game/Mathis/UI/UI_Event_Sacrifice.UI_Event_Sacrifice_C"))
                  (set `/Game/Mathis/UI/UI_Event_Sacrifice.Mine` self _returnvalue_7)
                  (`UserWidget.AddToViewport` _returnvalue_7 0)
                  (`|PlayAnimationTimeRange` _returnvalue_7 (`/Game/Mathis/UI/UI_Event_Sacrifice.Slide_Panel_Sacrifice` _returnvalue_7))
                  (elif (and (<= (`self.num event`) 65) (>= (`self.num event`) 51))
                    (bind _returnvalue_8 (`|CreateWidget` "/Game/Mathis/UI/UI_Event_SousProduction.UI_Event_SousProduction_C"))
                    (set `/Game/Mathis/UI/UI_Event_SousProduction.Mine` self _returnvalue_8)
                    (`UserWidget.AddToViewport` _returnvalue_8 0)
                    (`|PlayAnimationTimeRange` _returnvalue_8 (`/Game/Mathis/UI/UI_Event_SousProduction.Slide_Event_SousProduction` _returnvalue_8))
                    (elif (and (<= (`self.num event`) 50) (>= (`self.num event`) 31))
                      (bind _returnvalue_9 (`|CreateWidget` "/Game/Mathis/UI/UI_Event_Surproduction.UI_Event_Surproduction_C"))
                      (set `/Game/Mathis/UI/UI_Event_Surproduction.Mine` self _returnvalue_9)
                      (`UserWidget.AddToViewport` _returnvalue_9 0)
                      (`|PlayAnimationTimeRange` _returnvalue_9 (`/Game/Mathis/UI/UI_Event_Surproduction.Slide_Panel_Surproduction` _returnvalue_9)))))))))))))

(fn `NewFunction`)

(fn `Random Event`)

(fn `UserConstructionScript`)