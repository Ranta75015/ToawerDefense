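; Player pawn for a tower game with three factions (spirits, French, Indians), handling camera pan and zoom, mouse input, morale UI and pause menu.
; Every Tick it turns morale thresholds into gold bonuses on the Mine and French and Indian multipliers, updates the bars and prunes invalid towers.
; Delay-based events temporarily raise or lower gold, deactivate French or non-French towers, or boost or weaken both multipliers.
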(event `Key|MouseScrollDown`
  (params (Key :type "Key Structure"))
  (bind _springarm (`self.SpringArm`))
  (bind _targetarmlength (`SpringArmComponent.TargetArmLength` _springarm))
  ;[1 0.1645 0.9183] Camera Role
  (:`Pressed`
    (if (not (>= _targetarmlength (`self.Max dezoom`)))
      (set `SpringArmComponent.TargetArmLength` (+ 20.0 _targetarmlength) _springarm))))

(event `InputAxis|Move Forward / Backward`
  (params (AxisValue :type "Float (single-precision)"))
  ;[0.07743 1 0.9003] Mouvment
  (`self.K2_AddActorLocalOffset` (`KismetMathLibrary.MakeVector` (* AxisValue (`self.Cam Speed`)))))

(event `Update bar`
  (bind _ui (`self.ui`))
  (`/Game/Mathis/UI/UI_MoralBar.Get_Spirit_Moral_Bar_Percent` _ui (`KismetMathLibrary.Conv_IntToDouble` (`self.Humeur Phan`)) 0.0 (`KismetMathLibrary.Conv_IntToDouble` (`self.MaxHumeur Phan`)))
  (`/Game/Mathis/UI/UI_MoralBar.Get_French_Moral_Bar_Percent` _ui (`KismetMathLibrary.Conv_IntToDouble` (`self.Humeur Fr`)) 0.0 (`KismetMathLibrary.Conv_IntToDouble` (`self.MaxHumeur Fr`)))
  (`/Game/Mathis/UI/UI_MoralBar.Get_Indians_Moral_Bar_Percent` _ui (`KismetMathLibrary.Conv_IntToDouble` (`self.Humeur Ind`)) 0.0 (`KismetMathLibrary.Conv_IntToDouble` (`self.MaxHumeur Ind`))))

(event `InputAxis|Move Right / Left`
  (params (AxisValue :type "Float (single-precision)"))
  ;[0.07743 1 0.9003] Mouvment
  (`self.K2_AddActorLocalOffset` (`KismetMathLibrary.MakeVector` 0.0 (* (`self.Cam Speed`) AxisValue))))

(event `Key|MouseScrollUp`
  (params (Key :type "Key Structure"))
  (bind _springarm (`self.SpringArm`))
  (bind _targetarmlength (`SpringArmComponent.TargetArmLength` _springarm))
  ;[1 0.1645 0.9183] Camera Role
  (:`Pressed`
    (if (not (<= _targetarmlength (`self.Max zoom`)))
      (set `SpringArmComponent.TargetArmLength` (- _targetarmlength 20.0) _springarm))))

(event `self.ReceiveBeginPlay`
  (bind _returnvalue (`GameplayStatics.GetPlayerController` 0))
  (set `PlayerController.bShowMouseCursor` true _returnvalue)
  (set `PlayerController.bEnableClickEvents` true _returnvalue)
  (set `PlayerController.bEnableMouseOverEvents` true _returnvalue)
  (bind _returnvalue_2 (`|CreateWidget` "/Game/Mathis/UI/UI_MoralBar.UI_MoralBar_C"))
  (set `self.ui` _returnvalue_2)
  (set `/Game/Mathis/UI/UI_MoralBar.Mine` (`self.Mine`) _returnvalue_2)
  (`UserWidget.AddToViewport` _returnvalue_2 0))

(event `Boost gold`
  (bind _mine (`self.Mine`))
  (bind _mine_2 (`self.Mine`))
  (set `/Game/Valentin/BluePrint/GestionnaireEvent/BP_Mine.Bonus Gold` (+ (`/Game/Valentin/BluePrint/GestionnaireEvent/BP_Mine.Bonus Gold` _mine) 1) _mine)
  (`KismetSystemLibrary.Delay` 60.0)
  (set `/Game/Valentin/BluePrint/GestionnaireEvent/BP_Mine.Bonus Gold` (- (`/Game/Valentin/BluePrint/GestionnaireEvent/BP_Mine.Bonus Gold` _mine_2) 1) _mine_2))

(event `self.ReceiveTick`
  (params (DeltaSeconds :type "Float (single-precision)"))
  (bind _tour (`self.Tour`))
  (`self.Humeur modifieur`)
  (`self.Bonus gold humeur`)
  (`self.Update bar`)
  (for (_ _array_index) _tour
    (`/Engine/EditorBlueprintResources/StandardMacros.IsValid` (`|GetArrayItem` _tour _array_index)
      (:`Is Not Valid`
        (`KismetArrayLibrary.Array_Remove` _tour _array_index)
        (`|ExecutionSequence`
          (:`then_0`
            (if (< (`self.Humeur Phan`) 0)
              (set `self.Humeur Phan` 0)))
          (:`then_1`
            (if (< (`self.Humeur Fr`) 0)
              (set `self.Humeur Fr` 0)))
          (:`then_2`
            (if (< (`self.Humeur Ind`) 0)
              (set `self.Humeur Ind` 0))))))))

(event `DownBoost gold`
  (bind _mine (`self.Mine`))
  (bind _mine_2 (`self.Mine`))
  (set `/Game/Valentin/BluePrint/GestionnaireEvent/BP_Mine.Bonus Gold` (- (`/Game/Valentin/BluePrint/GestionnaireEvent/BP_Mine.Bonus Gold` _mine) 1) _mine)
  (`KismetSystemLibrary.Delay` 60.0)
  (set `/Game/Valentin/BluePrint/GestionnaireEvent/BP_Mine.Bonus Gold` (+ (`/Game/Valentin/BluePrint/GestionnaireEvent/BP_Mine.Bonus Gold` _mine_2) 1) _mine_2))

(event `Inactive french`
  (bind _tour (`self.Tour`))
  (bind _tour_2 (`self.Tour`))
  (for (_ _array_index) _tour
    (bind _output (`|GetArrayItem` _tour _array_index))
    (if (`/Game/Valentin/BluePrint/Tour/BP_TestTour.I'm french?` _output)
      (set `/Game/Valentin/BluePrint/Tour/BP_TestTour.I'm active?` false _output)))
  (`KismetSystemLibrary.Delay` 120.0)
  (for (_ _array_index_2) _tour_2
    (bind _output_2 (`|GetArrayItem` _tour_2 _array_index_2))
    (if (`/Game/Valentin/BluePrint/Tour/BP_TestTour.I'm french?` _output_2)
      (set `/Game/Valentin/BluePrint/Tour/BP_TestTour.I'm active?` true _output_2))))

(event `Humeur modifieur`
  (`|ExecutionSequence`
    (:`then_0`
      (if (> (`self.Humeur Phan`) 74)
        (set `self.gold phan` 1)
        (elif (> (`self.Humeur Phan`) 49)
          (set `self.gold phan` 0)
          (elif (> (`self.Humeur Phan`) 24)
            _))))
    (:`then_1`
      (if (> (`self.Humeur Fr`) 74)
        (set `self.Gold fr` 1)
        (if (not (`self.Boost Active?`))
          (set `self.Multiplicateur Fr` 1.5))
        (elif (> (`self.Humeur Fr`) 49)
          (set `self.Gold fr` 0)
          (if (not (`self.Boost Active?`))
            (set `self.Multiplicateur Fr` 1.0))
          (elif (> (`self.Humeur Fr`) 24)
            (if (not (`self.Boost Active?`))
              (set `self.Multiplicateur Fr` 0.75))))))
    (:`then_2`
      (if (> (`self.Humeur Ind`) 74)
        (set `self.Gold Ind` 1)
        (if (not (`self.Boost Active?`))
          (set `self.Multiplicateur Ind` 1.5))
        (elif (> (`self.Humeur Ind`) 49)
          (set `self.Gold Ind` 0)
          (if (not (`self.Boost Active?`))
            (set `self.Multiplicateur Ind` 1.0))
          (elif (> (`self.Humeur Ind`) 24)
            (if (not (`self.Boost Active?`))
              (set `self.Multiplicateur Ind` 0.75))))))))

(event `Inactive Indian`
  (bind _tour (`self.Tour`))
  (bind _tour_2 (`self.Tour`))
  (for (_ _array_index) _tour_2
    (bind _output (`|GetArrayItem` _tour_2 _array_index))
    (if (not (`/Game/Valentin/BluePrint/Tour/BP_TestTour.I'm french?` _output))
      (set `/Game/Valentin/BluePrint/Tour/BP_TestTour.I'm active?` false _output)))
  (`KismetSystemLibrary.Delay` 120.0)
  (for (_ _array_index_2) _tour
    (bind _output_2 (`|GetArrayItem` _tour _array_index_2))
    (if (not (`/Game/Valentin/BluePrint/Tour/BP_TestTour.I'm french?` _output_2))
      (set `/Game/Valentin/BluePrint/Tour/BP_TestTour.I'm active?` true _output_2))))

(event `InputAction|Pause`
  (params (Key :type "Key Structure"))
  (:`Pressed`
    (bind _returnvalue (`|CreateWidget` "/Game/Mathis/UI/UI_Pause.UI_Pause_C"))
    (`UserWidget.AddToViewport` _returnvalue 0)
    (`UserWidget.PlayAnimation` _returnvalue (`/Game/Mathis/UI/UI_Pause.Slide_Personnage` _returnvalue) 0.0 0 "Forward" 1.0 false)
    (`GameplayStatics.SetGamePaused` true)))

(event `Boost all`
  (if (`self.tower was boost?`)
    (set `self.Multiplicateur Ind` 2.0)
    (set `self.Multiplicateur Fr` 2.0)
    (else
      (set `self.Multiplicateur Ind` 0.5)
      (set `self.Multiplicateur Fr` 0.5)))
  (`KismetSystemLibrary.Delay` 180.0)
  (set `self.Boost Active?` false)
  (set `self.tower was boost?` false))

(fn `Bonus gold humeur`
  (set `/Game/Valentin/BluePrint/GestionnaireEvent/BP_Mine.Bonus humeur` (+ (`self.gold phan`) (`self.Gold fr`) (`self.Gold Ind`)) (`self.Mine`)))

(fn `UserConstructionScript`)