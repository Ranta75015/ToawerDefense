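; Test tower Blueprint that tracks enemies in range, shoots at the first one and displays its health on a widget bar.
; Actor overlap events add and remove BP_TestEnemie actors in a target list, and Tick prunes an invalid first entry.
; Each Tick also refreshes the UI_LifeFriends bar, rotates the body toward the first target and calls Fire, whose Delay paces BP_Amo spawns at the Mire component.
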(event `self.ReceiveActorEndOverlap`
  (params (OtherActor :type "Actor Object Reference"))
  (bind _asbp_test_enemie (cast `/Game/Valentin/BluePrint/BP_TestEnemie` OtherActor))
  (`KismetArrayLibrary.Array_RemoveItem` (`self.Liste ennemie`) _asbp_test_enemie))

(event `Updaet life`
  (params (DeltaSeconds :type "Float (single-precision)"))
  ;[0 1 0.2406] Mise a jour vie
  (bind _asui_life_friends (cast `/Game/Valentin/Ui/UI_LifeFriends` (`WidgetComponent.GetWidget` (`self.Life Bar`))))
  (`/Game/Valentin/Ui/UI_LifeFriends.Update Health bar` _asui_life_friends (`self.Life`) (`self.MinLife`) (`self.MaxLife`)))

(event `self.ReceiveActorBeginOverlap`
  (params (OtherActor :type "Actor Object Reference"))
  (bind _asbp_test_enemie (cast `/Game/Valentin/BluePrint/BP_TestEnemie` OtherActor))
  (`KismetArrayLibrary.Array_Add` (`self.Liste ennemie`) _asbp_test_enemie))

(event `self.ReceiveTick`
  (params (DeltaSeconds :type "Float (single-precision)"))
  (bind _liste_ennemie (`self.Liste ennemie`))
  (`self.Updaet life` 0.0)
  (`self.Folow targert`)
  (`self.fire`)
  (`/Engine/EditorBlueprintResources/StandardMacros.IsValid` (`|GetArrayItem` _liste_ennemie)
    (:`Is Not Valid`
      (`KismetArrayLibrary.Array_Remove` _liste_ennemie))))

(event `fire`
  (if (not (`KismetArrayLibrary.Array_IsEmpty` (`self.Liste ennemie`)))
    (`KismetSystemLibrary.Delay` 0.15)
    (`|SpawnActorFromClass` "/Game/Valentin/BluePrint/BP_Amo.BP_Amo_C" (`SceneComponent.K2_GetComponentToWorld` (`self.Mire`)) "Undefined" "OverrideRootScale" null null)))

(fn `Folow targert`
  (`/Engine/EditorBlueprintResources/StandardMacros.IsValid` (`|GetArrayItem` (`self.Liste ennemie`))
    (:`Is Valid`
      (`SceneComponent.K2_SetRelativeRotation` (`self.Corp`) (`KismetMathLibrary.FindLookAtRotation` (`SceneComponent.K2_GetComponentLocation` (`self.Corp`)) (`self.K2_GetActorLocation` (`|GetArrayItem` (`self.Liste ennemie`)))) false false))))

(fn `UserConstructionScript`)